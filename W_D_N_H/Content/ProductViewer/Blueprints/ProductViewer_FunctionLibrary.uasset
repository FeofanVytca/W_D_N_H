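; Function library for the Product Viewer with helpers for reading transforms stored in tags and building menu buttons.
; FindTagInfo finds the first array entry containing "Transform", splits it on "+" into location, rotation and scale, and returns a found flag, index and transform.
; MakeCustomMenuButton creates a MenuButton widget, binds the supplied event to it, sets its text, adds it to the given menu and returns it.
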(fn `FindTagInfo`
  (params (Array :type "Array of Name"))
  (returns (ExistingTagFound :type Boolean) (Index :type Integer) (ExistingTagTransform :type "Transform Structure"))
  (locals (TagFound :type Boolean) (TagIndex :type Integer) (FoundTransorm :type "Transform Structure"))
  (set `local.TagFound` false)
  (for (_array_element _array_index) Array
    (bind _returnvalue (`KismetStringLibrary.Conv_NameToString` _array_element))
    (bind _returnvalue_2 (`KismetStringLibrary.EqualEqual_StrStr` (`KismetStringLibrary.GetSubstring` _returnvalue (`KismetStringLibrary.FindSubstring` _returnvalue "Transform" true) 9) "Transform"))
    (if _returnvalue_2
      (`|ExecutionSequence`
        (:`then_0`
          (break))
        (:`then_1`
          (set `local.TagFound` _returnvalue_2)
          (set `local.TagIndex` _array_index)
          (bind _returnvalue_3 (`KismetStringLibrary.ParseIntoArray` (`KismetStringLibrary.Conv_NameToString` _array_element) "+"))
          (set `local.FoundTransorm` (`KismetMathLibrary.MakeTransform` (`KismetStringLibrary.Conv_StringToVector` (`|GetArrayItem` _returnvalue_3 1)) (`KismetStringLibrary.Conv_StringToRotator` (`|GetArrayItem` _returnvalue_3 2)) (`KismetStringLibrary.Conv_StringToVector` (`|GetArrayItem` _returnvalue_3 3))))))))
  (return (`local.TagFound`) (`local.TagIndex`) (`local.FoundTransorm`)))

(fn `MakeCustomMenuButton`
  (params (BindEventToClickedButton :type "Delegate (by ref)") (ButtonText :type Text) (CustomMenu :type "/Game/ProductViewer/Blueprints/Widgets/CustomMenu Object Reference"))
  (returns (CurrentButton :type "/Game/ProductViewer/Blueprints/Widgets/MenuButton Object Reference"))
  (bind _returnvalue (`|CreateWidget` "/Game/ProductViewer/Blueprints/Widgets/MenuButton.MenuButton_C"))
  (add `/Game/ProductViewer/Blueprints/Widgets/MenuButton.ClickedButton` _returnvalue BindEventToClickedButton)
  (add `/Game/ProductViewer/Blueprints/Widgets/MenuButton.DoIt` _returnvalue BindEventToClickedButton)
  (`TextBlock.SetText` (`/Game/ProductViewer/Blueprints/Widgets/MenuButton.Button_Text` _returnvalue) ButtonText)
  (`/Game/ProductViewer/Blueprints/Widgets/CustomMenu.AddButton` CustomMenu _returnvalue)
  (return _returnvalue))