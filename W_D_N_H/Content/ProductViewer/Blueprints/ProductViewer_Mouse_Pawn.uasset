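; Mouse-driven product viewer pawn that feeds input to inherited camera and actor manipulation functions.
; Drags orbit, pan or move tagged actors and the wheel dollies, while clicks restore transforms, fit view or set interest points.
; Hovering highlights interactive actors through custom depth, and holding Space opens a cursor menu to apply, isolate or remove X-ray.
; Input events enable Tick, which updates movement and calls DisableTick to avoid idle updates.
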(event `self.ReceiveBeginPlay`
  (bind _returnvalue (`GameplayStatics.GetPlayerController` 0))
  ;[0.2546 1 0.2921] Begin Play
  (`parent.ReceiveBeginPlay`)
  (`|ExecutionSequence`
    (:`then_0`
      (`KismetMaterialLibrary.SetScalarParameterValue` "/Game/ProductViewer/Materials/SelectableParams.SelectableParams" "SelectIntensity" 1.0)
      (`self.SetActorTickEnabled` true))
    (:`then_1`
      ;;[1 1 1] Setup the Input modes
      (`self.EnableInput` _returnvalue)
      (set `PlayerController.bEnableClickEvents` true _returnvalue)
      (set `PlayerController.bShowMouseCursor` true _returnvalue)
      (set `PlayerController.bEnableMouseOverEvents` true _returnvalue)
      (`Controller.SetIgnoreLookInput` _returnvalue true))
    (:`then_2`
      (for _array_element (`self.InterativeActors`)
        (`self.BindHighLightable` _array_element)))
    (:`then_4`
      (`self.CreateCustomMenu`)
      (`/Game/ProductViewer/Blueprints/ProductViewer_FunctionLibrary.MakeCustomMenuButton` (delegate `Bind_ApplyXray`) "Apply X Ray" (`self.CustomMenu`))
      (`/Game/ProductViewer/Blueprints/ProductViewer_FunctionLibrary.MakeCustomMenuButton` (delegate `Bind_IsolateXray`) "Isolate X Ray" (`self.CustomMenu`))
      (`/Game/ProductViewer/Blueprints/ProductViewer_FunctionLibrary.MakeCustomMenuButton` (delegate `Bind_RemoveXray`) "Remove X Ray" (`self.CustomMenu`)))))

(event `Bind_RemoveXray`
  ;[0.2546 1 0.2921] Begin Play
  (`self.RemoveXray`))

(event `Bind_ApplyXray`
  (bind _menu_highlightable_touchedactor (`self.Menu_HighLightable_TouchedActor`))
  ;[0.2546 1 0.2921] Begin Play
  (`/Engine/EditorBlueprintResources/StandardMacros.IsValid` _menu_highlightable_touchedactor
    (:`Is Valid`
      (`self.ApplyXray` _menu_highlightable_touchedactor))))

(event `Bind_IsolateXray`
  (bind _menu_highlightable_touchedactor (`self.Menu_HighLightable_TouchedActor`))
  ;[0.2546 1 0.2921] Begin Play
  (`/Engine/EditorBlueprintResources/StandardMacros.IsValid` _menu_highlightable_touchedactor
    (:`Is Valid`
      (`self.IsolateXray` _menu_highlightable_touchedactor))))

(event `BindHighLightable`
  (params (Actor :type "Actor Object Reference"))
  ;[0.2555 0.7775 1] Bind Highlightable
  (add `self.OnBeginCursorOver` Actor (delegate `HighLightOn`))
  (add `self.OnEndCursorOver` Actor (delegate `HighLightOff`)))

(event `HighLightOn` :!signature `self.OnBeginCursorOver`
  (params (TouchedActor :type "Actor Object Reference"))
  ;[0.2555 0.7775 1] Bind Highlightable
  (set `self.HighLightable_TouchedActor` TouchedActor)
  (if (not (or (`self.IsObjectTranslating`) (`self.ShowMenu`)))
    (`self.SetCustomDepth` TouchedActor true)))

(event `HighLightOff` :!signature `self.OnEndCursorOver`
  (params (TouchedActor :type "Actor Object Reference"))
  ;[0.2555 0.7775 1] Bind Highlightable
  (if (not (or (`self.IsObjectTranslating`) (`self.ShowMenu`)))
    (`self.SetCustomDepth` TouchedActor))
  (set `self.HighLightable_TouchedActor` null))

(event `UpdateMouseInput`
  (bind (_deltax _deltay) (`PlayerController.GetInputMouseDelta` (`GameplayStatics.GetPlayerController` 0)))
  ;[0.2555 0.7775 1] MouseInputs
  (set `self.SwipeInputDelta` (`KismetMathLibrary.MakeVector2D` _deltax _deltay))
  (set `self.DollyInput` (`self.GetInputAxisKeyValue`)))

(event `self.ReceiveTick`
  (params (DeltaSeconds :type "Float (single-precision)"))
  (bind (_locationx _locationy) (`PlayerController.GetMousePosition` (`GameplayStatics.GetPlayerController` 0)))
  ;[1 0.1326 0.09279] Update every frame only  when Interacting
  (`|ExecutionSequence`
    (:`then_0`
      (if (not (`self.ShowMenu`))
        (`self.UpdateMouseInput`)
        (`self.PanCamera` (`self.SwipeInputDelta`))
        (`self.OrbitCamera`)
        (`self.CameraDolly`)
        (`self.TranslateActor` (`self.HitModel`) (`KismetMathLibrary.MakeVector2D` _locationx _locationy))))
    (:`then_1`
      (`self.DisableTick` true))))

(event `Key|RightMouseButton`
  (params (Key :type "Key Structure"))
  (bind (_locationx _locationy) (`PlayerController.GetMousePosition` (`GameplayStatics.GetPlayerController` 0)))
  (bind _returnvalue (`KismetMathLibrary.MakeVector2D` _locationx _locationy))
  ;[1 0.8299 0.2633] Rotate
  (:`Pressed`
    (`self.SetActorTickEnabled` true)
    (set `self.StartInteractingLocation` _returnvalue)
    (`self.getHitLoc_Model` (`|MakeArray` "Interact" :!type "Name"))
    (set `self.IsOrbiting` true))
  (:`Released`
    (set `self.StopInteractingLocation` _returnvalue)
    (if (== (`self.StartInteractingLocation`) (`self.StopInteractingLocation`) :`ErrorTolerance` 0.01)
      (`self.RestoreInitialTransform`))
    (set `self.HitModel` null)
    (set `self.IsOrbiting` false)))

(event `Key|MiddleMouseButton`
  (params (Key :type "Key Structure"))
  (bind (_locationx _locationy) (`PlayerController.GetMousePosition` (`GameplayStatics.GetPlayerController` 0)))
  (bind _returnvalue (`KismetMathLibrary.MakeVector2D` _locationx _locationy))
  ;[1 0.8299 0.2633] Translate
  (:`Pressed`
    (if (not (`self.ShowMenu`))
      (`self.SetActorTickEnabled` true)
      (set `self.IsPanning` true)
      (set `self.StartInteractingLocation` _returnvalue)
      (bind _out (`self.getHitLoc_Model` (`|MakeArray` "Interact" :!type "Name")))
      (set `self.canZoomSeleted` _out)))
  (:`Released`
    (if (not (`self.ShowMenu`))
      (set `self.IsPanning` false)
      (set `self.StopInteractingLocation` _returnvalue)
      (if (`self.canZoomSeleted`)
        (if (== (`self.StartInteractingLocation`) (`self.StopInteractingLocation`) :`ErrorTolerance` 0.01)
          (`self.SetFitView`))))))

(event `Key|LeftMouseButton` :consume false
  (params (Key :type "Key Structure"))
  (bind _showmenu (`self.ShowMenu`))
  (bind (_locationx _locationy) (`PlayerController.GetMousePosition` (`GameplayStatics.GetPlayerController` 0)))
  (bind _returnvalue (`KismetMathLibrary.MakeVector2D` _locationx _locationy))
  ;[1 0.8299 0.2633] Set Orbit / Move Actor
  (:`Pressed`
    (if (not _showmenu)
      (set `self.StartInteractingLocation` _returnvalue)
      (if (and (`self.IsInterestPointAnimDone`) (not (`self.IsFitView`)))
        (bind (_out _location _tagfound) (`self.getHitLoc_Model` (`|MakeArray` "Interact" "Teleport" :!type "Name")))
        (set `self.hitFound` _out)
        (if (== _tagfound "Interact")
          (set `self.IsObjectTranslating` true)
          (`self.SetActorTickEnabled` true)))))
  (:`Released`
    (if (not _showmenu)
      (set `self.StopInteractingLocation` _returnvalue)
      (if (and (not (`self.IsOrbiting`)) (`self.IsInterestPointAnimDone`))
        (if (== (`self.StartInteractingLocation`) (`self.StopInteractingLocation`) :`ErrorTolerance` 0.01)
          (if (`self.hitFound`)
            (`self.SetCameraInterestPoint`))))
      (set `self.IsObjectTranslating` false))))

(event `Key|MouseScrollDown`
  (params (Key :type "Key Structure"))
  ;[1 0.8299 0.2633] Zoom Enabled
  (:`Pressed`
    (`self.SetActorTickEnabled` true :!label _label)
    (set `self.IsDolly` true))
  (:`Released`
    (set `self.IsDolly` false :!label _label_2)))

(event `Key|MouseScrollUp`
  (params (Key :type "Key Structure"))
  ;[1 0.8299 0.2633] Zoom Enabled
  (:`Pressed`
    (goto _label))
  (:`Released`
    (goto _label_2)))

(event `Key|SpaceBar` :consume false
  (params (Key :type "Key Structure"))
  (bind (_locationx _locationy) (`PlayerController.GetMousePosition` (`GameplayStatics.GetPlayerController` 0)))
  ;[1 0.8299 0.2633] ManageXray Interface
  (:`Pressed`
    (set `self.ShowMenu` true)
    (set `self.Menu_HighLightable_TouchedActor` (`self.HighLightable_TouchedActor`))
    (`/Game/ProductViewer/Blueprints/Widgets/CustomMenu.MakeButtonAllEnable` (`self.CustomMenu`))
    (`UserWidget.SetPositionInViewport` (`self.CustomMenu`) (+ (`KismetMathLibrary.MakeVector2D` _locationx _locationy) (-50.0 -30.0)) true)
    (`Widget.SetVisibility` (`self.CustomMenu`) "Visible"))
  (:`Released`
    (set `self.ShowMenu` false)
    (`Widget.SetVisibility` (`self.CustomMenu`) "Collapsed")
    (if (not (== (`self.Menu_HighLightable_TouchedActor`) (`self.HighLightable_TouchedActor`)))
      (`self.SetCustomDepth` (`self.Menu_HighLightable_TouchedActor`)))))

(fn `getHitLoc_Model`
  (params (InteractiveTag :type "Array of Name (by ref)") (Hit :type "HitResult Structure") (HitReturn :type Boolean) (ExcludeModels :type Boolean))
  (returns (Out :type Boolean) (Location :type "Vector Structure") (TagFound :type Name))
  (bind (_hitresult _returnvalue) (`PlayerController.GetHitResultUnderCursorForObjects` (`GameplayStatics.GetPlayerController` 0) (`|MakeArray` "ObjectTypeQuery1" "ObjectTypeQuery2" :!type "EObjectTypeQuery Enum") true))
  (bind (_out _location _tagfound) (`parent.getHitLoc_Model` InteractiveTag _hitresult _returnvalue false))
  (return _out _location _tagfound))

(fn `UserConstructionScript`)